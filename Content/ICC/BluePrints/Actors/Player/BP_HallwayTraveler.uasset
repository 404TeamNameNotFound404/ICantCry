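; BP_HallwayTraveler is a trigger actor that plays a room fade-out sequence when its box component is overlapped, if fading is enabled.
; On overlap it disables the first player character's input and plays the RoomFadeOut Level Sequence through a player created at runtime.
; Timed delays restore input, then destroy the spawned sequence actor.
; The overlapping actor is not checked, and the graph itself moves no one.
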(event `self.BoxComponent.OnComponentBeginOverlap`
  (params (OverlappedComponent :type "PrimitiveComponent Object Reference") (OtherActor :type "Actor Object Reference") (OtherComp :type "PrimitiveComponent Object Reference") (OtherBodyIndex :type Integer) (bFromSweep :type Boolean) (SweepResult :type "HitResult Structure (by ref)"))
  (bind _returnvalue (`GameplayStatics.GetPlayerController` 0))
  (bind _returnvalue_2 (`GameplayStatics.GetPlayerCharacter` 0))
  (if (`self.bEnableFade`)
    (`self.DisableInput` _returnvalue_2 _returnvalue)
    (bind (_outactor _returnvalue_3) (`LevelSequencePlayer.CreateLevelSequencePlayer` "/Game/ICC/Cinematics/Global/RoomFadeOut.RoomFadeOut"))
    (`MovieSceneSequencePlayer.Play` _returnvalue_3)
    (`KismetSystemLibrary.Delay` 0.9)
    (`self.EnableInput` _returnvalue_2 _returnvalue)
    (`KismetSystemLibrary.Delay` 0.4)
    (`self.K2_DestroyActor` _outactor)))

(fn `UserConstructionScript`)